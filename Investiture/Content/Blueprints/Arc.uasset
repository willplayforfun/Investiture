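; Arc actor that draws an arched trail of beam segments in its local space, with a settable color applied at BeginPlay.
; BuildArc clears BeamTrail, then links points from GetPoint, transformed by the actor transform.
; GetPoint moves linearly along X to Distance and shapes Z with a cosine scaled by Height.
; BuildArc's EndHeight has no effect because its Lerp alpha is fixed at zero.
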(event EventBeginPlay
  (CallFunction|SetColor (Variables|Default|GetColor)))

(event Collision|EventActorBeginOverlap
  (params (OtherActor :type Actor%20Object%20Reference)))

(event EventTick
  (params (DeltaSeconds :type Float%20%28single-precision%29)))

(fn ConstructionScript)

(fn BuildArc
  (params (EndHeight :type Float%20%28single-precision%29))
  (bind _returnvalue (Math|Float|Lerp 0.0 EndHeight 0.0))
  (bind _height (Variables|Default|GetHeight))
  (bind _distance (Variables|Default|GetDistance))
  (bind _returnvalue_2 (+ _returnvalue _height))
  (CallFunction|ClearArc)
  (for _index (range 0 (Variables|Default|GetNumSegments))
    (Default|AddBeam (Variables|Default|GetBeamTrail) (Math|Transform|TransformLocation (Transformation|GetActorTransform) (CallFunction|GetPoint _distance _returnvalue_2 (LocalVariables|GetLastT))) (Math|Transform|TransformLocation (Transformation|GetActorTransform) (CallFunction|GetPoint _distance _returnvalue_2 (/ (Math|Conversions|ToFloat(Integer) _index) (Math|Conversions|ToFloat(Integer) (Variables|Default|GetNumSegments))))))
    (LocalVariables|SetLastT (/ (Math|Conversions|ToFloat(Integer) _index) (Math|Conversions|ToFloat(Integer) (Variables|Default|GetNumSegments)))))
  (Development|PrintString "Built arc!" true true "(R=0.000000,G=0.660000,B=1.000000,A=1.000000)" 4.0))

(fn ClearArc
  (Default|ClearBeams (Variables|Default|GetBeamTrail)))

(fn GetPoint
  (params (Distance :type Float%20%28single-precision%29) (Height :type Float%20%28single-precision%29) (Time :type Float%20%28single-precision%29))
  (return (Math|Vector|MakeVector (Math|Float|Lerp 0.0 Distance Time) 0.0 (* Height (Math|Trig|Cos(Degrees) (Math|Float|Lerp -9e+01 9e+01 Time))))))

(fn SetColor
  (params (New%20Color :type Linear%20Color%20Structure))
  (bind _output_get (Variables|Default|SetColor New%20Color))
  (Default|SetColor (Variables|Default|GetBeamTrail) _output_get))
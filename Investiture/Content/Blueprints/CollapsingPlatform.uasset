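; Collapsing platform actor that flags when the first-person character overlaps it and can cycle its Cube vertically.
; Reset restores the start transform, clears the flag and schedules MoveDownAndUp, a repeating timer that plays the down timeline and sets a delayed follow-up event.
; Up and down timelines teleport the Cube by scaled offsets.
; Collapse alters constraint mode and disables step-up after a post-reset grace period, but nothing here calls it.
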(event Custom|AnimateMoveDown
  (bind _offset (Timeline|MoveDownTimeline PlayFromStart)
    (:Update
      (Transformation|SetWorldLocation (Variables|Default|GetCube) (+ (* _offset (Variables|Default|GetMoveHeight)) (.Location (Math|Transform|BreakTransform (Variables|Default|GetStartTransform)))) false true))))

(event Custom|AnimateMoveUp
  (bind _offset (Timeline|MoveUpTimeline PlayFromStart)
    (:Update
      (Transformation|SetWorldLocation (Variables|Default|GetCube) (+ (* _offset (Variables|Default|GetMoveHeight)) (.Location (Math|Transform|BreakTransform (Variables|Default|GetStartTransform)))) false true))))

(event EventBeginPlay)

(event Collision|EventActorBeginOverlap
  (params (OtherActor :type Actor%20Object%20Reference))
  (if (not (Variables|Default|GetTriggered))
    (if (== (Utilities|GetClass OtherActor) "/Game/Blueprints/FirstPersonCharacter.FirstPersonCharacter_C")
      (Variables|Default|SetTriggered true))))

(event EventTick
  (params (DeltaSeconds :type Float%20%28single-precision%29)))

(fn ConstructionScript
  (Variables|Default|SetStartTransform (Transformation|GetWorldTransform (Variables|Default|GetCube))))

(fn Collapse
  (if (>= (- (Utilities|Time|GetTimeSeconds) (Variables|Default|GetResetTime)) "0.5f")
    (Class|PrimitiveComponent|SetConstraintMode (Variables|Default|GetCube) "None")
    (Variables|/Script/Engine.PrimitiveComponent|SetCanCharacterStepUpOn (Variables|Default|GetCube) "ECB_No")))

(fn Reset
  (Transformation|SetWorldTransform (Variables|Default|GetCube) (Variables|Default|GetStartTransform) false true)
  (Variables|Default|SetTriggered false)
  (Variables|/Script/Engine.PrimitiveComponent|SetCanCharacterStepUpOn (Variables|Default|GetCube) "ECB_Yes")
  (Variables|Default|SetResetTime (Utilities|Time|GetTimeSeconds))
  (Utilities|Time|ClearTimerbyFunctionName self "MoveDownAndUp")
  (Utilities|Time|SetTimerbyFunctionName self "MoveDownAndUp" (+ (Variables|Default|GetMovePeriod) (Variables|Default|GetMoveTimeOffset))))

(fn MoveDownandUp
  (CallFunction|AnimateMoveDown)
  (Utilities|Time|SetTimerbyEvent (EventDispatchers|CreateEvent :!event Custom|AnimateMoveUp) (/ (Variables|Default|GetMovePeriod) 3.0))
  (Utilities|Time|SetTimerbyFunctionName self "MoveDownAndUp" (Variables|Default|GetMovePeriod)))
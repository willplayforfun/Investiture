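; CubeSpawner is an actor that spawns a single Cube at its own transform and launches it.
; Spawn destroys any previous cube, stores the new one, pushes its static mesh with a force from SpawnVelocity rotated into the spawner's local space, and prints a debug message.
; Reset destroys the current cube and respawns only if SpawnAtStart is set.
; The event graph is empty, so neither function is triggered from within this Blueprint.
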(event EventBeginPlay)

(event Collision|EventActorBeginOverlap
  (params (OtherActor :type Actor%20Object%20Reference)))

(event EventTick
  (params (DeltaSeconds :type Float%20%28single-precision%29)))

(fn ConstructionScript)

(fn Spawn
  (if (Utilities|IsValid (Variables|Default|GetSpawnedCube))
    (Actor|DestroyActor (Variables|Default|GetSpawnedCube)))
  (bind _returnvalue (Game|SpawnActorfromClass "/Game/Blueprints/Cube.Cube_C" (Transformation|GetActorTransform) "AdjustIfPossibleButAlwaysSpawn" 0 0))
  (bind _output_get (Variables|Default|SetSpawnedCube _returnvalue))
  (Physics|AddForce (Variables|/Game/Blueprints/Cube.Cube_C|GetStaticMesh _output_get) (Math|Transform|TransformDirection (Transformation|GetActorTransform) (Variables|Default|GetSpawnVelocity)) "None" false)
  (Development|PrintString (Utilities|String|Append (Utilities|GetObjectName self) " spawned a cube")))

(fn Reset
  (bind _spawnedcube (Variables|Default|GetSpawnedCube))
  (if (Utilities|IsValid _spawnedcube)
    (Actor|DestroyActor _spawnedcube))
  (if (Variables|Default|GetSpawnAtStart)
    (CallFunction|Spawn)))
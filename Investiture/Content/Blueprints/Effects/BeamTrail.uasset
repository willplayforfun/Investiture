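; BeamTrail is an effect component that draws a trail from beam particle segments between pairs of positions supplied by its caller.
; AddBeam spawns a persistent emitter per segment, sets its beam source and target points, tints it with BeamColor and stores it in Beams.
; SetColor, also applied at BeginPlay, retints every stored beam, and ClearBeams destroys them all and empties the array.
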(event EventBeginPlay
  (CallFunction|SetColor (Variables|Default|GetBeamColor)))

(event EventTick
  (params (DeltaSeconds :type Float%20%28single-precision%29)))

(fn AddBeam
  (params (PreviousPos :type Vector) (NewPos :type Vector))
  (bind _returnvalue (+ PreviousPos "0, 0, 0"))
  (bind _returnvalue_2 (Effects|SpawnEmitteratLocation (Variables|Default|GetParticleSystem) _returnvalue "0, 0, 0" "1.000000,1.000000,1.000000" false))
  (Class|ParticleSystemComponent|SetBeamTargetPoint (stale _returnvalue) 0 (+ NewPos "0, 0, 0"))
  (Class|ParticleSystemComponent|SetBeamSourcePoint (stale _returnvalue) 0 _returnvalue)
  (Effects|Components|ParticleSystem|SetColorParameter _returnvalue_2 "Color" (Variables|Default|GetBeamColor))
  (Utilities|Array|Add (Variables|Default|GetBeams) _returnvalue_2))

(fn ClearBeams
  (for _array_element (Variables|Default|GetBeams)
    (Components|DestroyComponent _array_element))
  (Utilities|Array|Clear (Variables|Default|GetBeams)))

(fn SetColor
  (params (New%20Color :type Linear%20Color%20Structure))
  (bind _output_get (Variables|Default|SetBeamColor New%20Color))
  (for _array_element (Variables|Default|GetBeams)
    (Effects|Components|ParticleSystem|SetColorParameter _array_element "Color" _output_get)))
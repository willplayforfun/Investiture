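; Floor button actor that lights four point lights and broadcasts OnActivate when an actor of exactly its AllowType class overlaps it.
; End overlap releases it only for FirstPersonCharacter, regardless of AllowType, turning the lights off and broadcasting OnDeactivate with an Instantaneous flag.
; Reset clears the Cubes array, which nothing here fills, and releases instantly.
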(event EventBeginPlay
  (CallFunction|SetLights false))

(event Collision|EventActorBeginOverlap
  (params (OtherActor :type Actor%20Object%20Reference))
  (if (== (Utilities|GetClass OtherActor) (Variables|Default|GetAllowType))
    (CallFunction|Press OtherActor)))

(event Collision|EventActorEndOverlap
  (params (OtherActor :type Actor%20Object%20Reference))
  (if (== (Utilities|GetClass OtherActor) "/Game/Blueprints/FirstPersonCharacter.FirstPersonCharacter_C")
    (CallFunction|Release false)))

(event EventTick
  (params (DeltaSeconds :type Float%20%28single-precision%29)))

(fn ConstructionScript)

(fn Release
  (params (Instantaneous :type Boolean))
  (CallFunction|SetLights false)
  (Default|CallOnDeactivate Instantaneous))

(fn Reset
  (Utilities|Set|Clear (Variables|Default|GetCubes))
  (CallFunction|Release true))

(fn SetLights
  (params (Visible :type Boolean))
  (Rendering|SetVisibility (Variables|Default|GetPointLight) Visible false)
  (Rendering|SetVisibility (Variables|Default|GetPointLight1) Visible false)
  (Rendering|SetVisibility (Variables|Default|GetPointLight2) Visible false)
  (Rendering|SetVisibility (Variables|Default|GetPointLight3) Visible false))

(fn Press
  (params (Actor :type Actor%20Object%20Reference))
  (CallFunction|SetLights true)
  (Default|CallOnActivate))
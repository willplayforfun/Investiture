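; LayoutButton is a layout placeholder that spawns a GroundButton at its world transform and can link it to a door.
; Spawn always creates the button regardless of collision and stores it in SpawnedButton, which Clear destroys if still valid.
; BindToDoor passes the spawned button, cast to GroundButton, to the given door's AttachToButton.
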(event EventBeginPlay)

(event EventTick
  (params (DeltaSeconds :type Float%20%28single-precision%29)))

(fn Spawn
  (bind _returnvalue (Game|SpawnActorfromClass "/Game/Blueprints/LevelElements/GroundButton.GroundButton_C" (Transformation|GetWorldTransform) "AlwaysSpawn" 0 0))
  (Variables|Default|SetSpawnedButton _returnvalue))

(fn Clear
  (bind _spawnedbutton (Variables|Default|GetSpawnedButton))
  (Utilities|IsValid _spawnedbutton
    (:Is%20Valid
      (Actor|DestroyActor _spawnedbutton))))

(fn BindtoDoor
  (params (Door :type Moving%20Door%20Object%20Reference))
  (Default|AttachtoButton Door (.AsGround%20Button (Utilities|Casting|CastToGroundButton (Variables|Default|GetSpawnedButton)))))
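; Socket component for procedural level generation that spawns a LevelLayout piece at its own transform.
; Spawn picks the piece class from the layout type, randomizing regular pieces within tiers gated by the allowed lives.
; A debug-drawn line trace to the piece's end marker destroys it and reports failure on a hit.
; Clear removes the piece and its obstacles, while cost getters return recursive jump and speed totals from the parent ObstaclePath.
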(event EventBeginPlay)

(event EventTick
  (params (DeltaSeconds :type Float%20%28single-precision%29)))

(fn Spawn
  (params (TotalAllowedLives :type Integer) (LayoutType :type LayoutType%20Enum :default "NewEnumerator0"))
  (bind _returnvalue (Game|SpawnActorfromClass (Utilities|Select :Index (Variables|Default|GetLayoutType) :NewEnumerator0 (Utilities|Select :Index (Math|Integer|Min(Integer) (Math|Random|RandomIntegerinRange 1 TotalAllowedLives) 2) :Option%200 0 :Option%201 (Utilities|Select :Index (Math|Random|RandomInteger 3) :Option%200 "/Game/Blueprints/Layouts/LayoutPiece_Button.LayoutPiece_Button_C" :Option%201 "/Game/Blueprints/Layouts/LayoutPiece_T.LayoutPiece_T_C" :Option%202 "/Game/Blueprints/Layouts/LayoutPiece_BoxGate.LayoutPiece_BoxGate_C") :Option%202 (Utilities|Select :Index (Math|Random|RandomInteger 2) :Option%200 "/Game/Blueprints/Layouts/LayoutPiece_BoxPuzzle.LayoutPiece_BoxPuzzle_C" :Option%201 "/Game/Blueprints/Layouts/LayoutPiece_Gate.LayoutPiece_Gate_C")) :NewEnumerator1 "/Game/Blueprints/Layouts/LayoutPiece_BoxSpawn.LayoutPiece_BoxSpawn_C" :NewEnumerator2 "/Game/Blueprints/Layouts/LayoutPiece_BoxButton.LayoutPiece_BoxButton_C") (Transformation|GetWorldTransform) "AlwaysSpawn" 0 0))
  (bind _output_get (Variables|Default|SetSpawnedLayout (.AsLevel%20Layout (Utilities|Casting|CastToLevelLayout _returnvalue))))
  ;[1 1 1] Remove if it collides with another layout piece
  (bind _returnvalue_2 (Collision|LineTraceByChannel (Transformation|GetWorldLocation) (Transformation|GetWorldLocation (Variables|/Game/Blueprints/Layouts/LevelLayout.LevelLayout_C|GetLineTraceEnd _output_get)) "TraceTypeQuery1" false (Utilities|Array|MakeArray _output_get) "ForDuration" true "(R=0.000000,G=1.000000,B=0.225423,A=1.000000)" "(R=1.000000,G=0.107998,B=0.000000,A=1.000000)" 1e+01))
  (if _returnvalue_2
    (Actor|DestroyActor (Variables|Default|GetSpawnedLayout))
    (return false)
    (else
      (return true))))

(fn Clear
  (bind _spawnedlayout (Variables|Default|GetSpawnedLayout))
  (Utilities|IsValid _spawnedlayout
    (:Is%20Valid
      (Default|ClearObstacles _spawnedlayout)
      (Actor|DestroyActor _spawnedlayout))))

(fn GetParentPath
  (bind _asobstacle_path (Utilities|Casting|CastToObstaclePath (Transformation|GetAttachParent))
    (:then
      (return _asobstacle_path))
    (:CastFailed
      (return 0))))

(fn GetJumpCostto
  (bind _path (CallFunction|GetParentPath))
  (Utilities|IsValid _path
    (:Is%20Valid
      (bind _jump (Default|GetRecursiveJump _path))
      (LocalVariables|SetRecursiveJump _jump))
    (:Is%20Not%20Valid
      _))
  (return (LocalVariables|GetRecursiveJump)))

(fn GetSpeedCostto
  (bind _path (CallFunction|GetParentPath))
  (Utilities|IsValid _path
    (:Is%20Valid
      (bind _speed (Default|GetRecursiveSpeed _path))
      (LocalVariables|SetRecursiveSpeed _speed))
    (:Is%20Not%20Valid
      _))
  (return (LocalVariables|GetRecursiveSpeed)))
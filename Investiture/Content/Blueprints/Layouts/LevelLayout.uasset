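; Procedural level layout piece that fills itself with jump, speed and strength obstacles, door buttons and nested sub-layouts for a puzzle.
; Populate randomly builds obstacles on its ObstaclePaths, then recursively spawns layouts at sockets within a randomly divided lives budget.
; It totals required stats across nesting, binds buttons to the puzzle's moving door and returns lives used.
; ClearObstacles resets paths, buttons and sockets; the endpoint-counting construction logic is disconnected.
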(fn ConstructionScript)

(fn GetStart
  (return (Transformation|GetWorldLocation (Variables|Default|GetStart))))

(fn GetEnd
  (return (Transformation|GetWorldLocation (Variables|Default|GetEnd))))

(fn GetDoor
  (return (Transformation|GetWorldTransform (Variables|Default|GetDoor))))

(fn Populate
  (params (Puzzle :type Procedural%20Puzzle%20Object%20Reference) (TotalAllowedLives :type Integer))
  (Utilities|FlowControl|Sequence
    (:then_0
      (for _array_element (Actor|GetComponentsByClass "/Game/Blueprints/Layouts/ObstaclePath.ObstaclePath_C")
        (Default|ClearObstacle _array_element)
        ;[1 1 1] Restrict obstacle types
        (Utilities|Array|Clear (LocalVariables|GetAllowedTypes))
        (if (Variables|/Game/Blueprints/Layouts/ObstaclePath.ObstaclePath_C|GetAllowJump _array_element)
          (Utilities|Array|Add (LocalVariables|GetAllowedTypes) 0))
        (if (Variables|/Game/Blueprints/Layouts/ObstaclePath.ObstaclePath_C|GetAllowSpeed _array_element)
          (Utilities|Array|Add (LocalVariables|GetAllowedTypes) 1))
        (if (Variables|/Game/Blueprints/Layouts/ObstaclePath.ObstaclePath_C|GetAllowStrength _array_element)
          (Utilities|Array|Add (LocalVariables|GetAllowedTypes) 2))
        (switch int (Math|Random|RandomInteger (Utilities|Array|Length (LocalVariables|GetAllowedTypes)))
          (:Default
            ;[1 1 1] Create obstacles
            (Development|PrintString "Invalid exec path while Populating level layout" true true "(R=1.000000,G=0.000000,B=0.078817,A=1.000000)" 5.0))
          (:0
            (bind _jumpvalue (Default|BuildJumpObstacle _array_element))
            (Development|PrintString (Utilities|String|Append "Spawned jump obstacle requiring " (Utilities|String|ToString(Integer) _jumpvalue)) true true "(R=0.000000,G=0.660000,B=1.000000,A=1.000000)" 5.0))
          (:1
            (bind _speedvalue (Default|BuildSpeedObstacle _array_element))
            (Development|PrintString (Utilities|String|Append "Spawned speed obstacle for requiring " (Utilities|String|ToString(Integer) _speedvalue)) true true "(R=0.000000,G=0.660000,B=1.000000,A=1.000000)" 5.0))
          (:2
            (bind _strengthvalue (Default|BuildStrengthObstacle _array_element))
            (Development|PrintString (Utilities|String|Append "Spawned strength obstacle for requiring " (Utilities|String|ToString(Integer) _strengthvalue)) true true "(R=0.000000,G=0.660000,B=1.000000,A=1.000000)" 5.0))))
      ;[1 1 1] Find stats needed for spawned obstacles (accounts for nesting)
      (for _array_element_2 (Actor|GetComponentsByClass "/Game/Blueprints/Layouts/ObstaclePath.ObstaclePath_C")
        (Utilities|FlowControl|Sequence
          (:then_0
            (bind _jump (Default|GetRecursiveJump _array_element_2))
            (LocalVariables|SetTotalJump (+ (LocalVariables|GetTotalJump) _jump)))
          (:then_1
            (bind _speed (Default|GetRecursiveSpeed _array_element_2))
            (LocalVariables|SetTotalSpeed (+ (LocalVariables|GetTotalSpeed) _speed)))
          (:then_2
            (bind _strength (Default|GetRecursiveStrength _array_element_2))
            (LocalVariables|SetTotalStrength (+ (LocalVariables|GetTotalStrength) _strength))))))
    (:then_1
      ;[1 1 1] Recurse
      (LocalVariables|SetLivesLeft (- TotalAllowedLives (Variables|Default|GetNumEndPoints)))
      (for _array_element_3 (Actor|GetComponentsByClass "/Game/Blueprints/Layouts/LayoutLayoutSocket.LayoutLayoutSocket_C")
        (if (> (LocalVariables|GetLivesLeft) 0)
          (bind _output_get (LocalVariables|Settemp_livesforrecursivelayout (Math|Random|RandomIntegerinRange 1 (LocalVariables|GetLivesLeft))))
          (bind _success (Default|Spawn _array_element_3 _output_get))
          (if _success
            (bind _livesused (CallFunction|Populate (Variables|/Game/Blueprints/Layouts/LayoutLayoutSocket.LayoutLayoutSocket_C|GetSpawnedLayout _array_element_3) Puzzle _output_get))
            (LocalVariables|SetLivesLeft (- (LocalVariables|GetLivesLeft) _livesused))
            (LocalVariables|SetTotalJump (+ (LocalVariables|GetTotalJump) (Variables|LevelLayout_C|GetSumJump (Variables|/Game/Blueprints/Layouts/LayoutLayoutSocket.LayoutLayoutSocket_C|GetSpawnedLayout _array_element_3))))
            (LocalVariables|SetTotalSpeed (+ (LocalVariables|GetTotalSpeed) (Variables|LevelLayout_C|GetSumSpeed (Variables|/Game/Blueprints/Layouts/LayoutLayoutSocket.LayoutLayoutSocket_C|GetSpawnedLayout _array_element_3))))
            (LocalVariables|SetTotalStrength (+ (LocalVariables|GetTotalStrength) (Variables|LevelLayout_C|GetSumStrength (Variables|/Game/Blueprints/Layouts/LayoutLayoutSocket.LayoutLayoutSocket_C|GetSpawnedLayout _array_element_3))))
            (else
              (Rendering|Debug|DrawDebugSphere (Transformation|GetWorldLocation _array_element_3) 1e+02 12 "(R=1.000000,G=0.058081,B=0.000000,A=1.000000)" 1e+01 1e+01)
              (Development|PrintString "Layout placement failed!" true true "(R=1.000000,G=0.000000,B=0.106418,A=1.000000)" 1e+01))))))
    (:then_2
      (Variables|Default|SetSumJump (LocalVariables|GetTotalJump))
      (Variables|Default|SetSumSpeed (LocalVariables|GetTotalSpeed))
      (Variables|Default|SetSumStrength (LocalVariables|GetTotalStrength)))
    (:then_3
      ;[1 1 1] Connect Buttons and Doors
      (for _array_element_4 (Actor|GetComponentsByClass "/Game/Blueprints/Layouts/LayoutButton.LayoutButton_C")
        (Default|Clear _array_element_4)
        (Default|Spawn _array_element_4)
        (Default|BindtoDoor _array_element_4 (Variables|/Game/Blueprints/ProceduralPuzzle.ProceduralPuzzle_C|GetMovingDoor Puzzle))))
    (:then_4
      (return (- TotalAllowedLives (LocalVariables|GetLivesLeft))))))

(fn ClearObstacles
  (Utilities|FlowControl|Sequence
    (:then_0
      (for _array_element (Actor|GetComponentsByClass "/Game/Blueprints/Layouts/ObstaclePath.ObstaclePath_C")
        (Default|ClearObstacle _array_element)))
    (:then_1
      (for _array_element_2 (Actor|GetComponentsByClass "/Game/Blueprints/Layouts/LayoutButton.LayoutButton_C")
        (Default|Clear _array_element_2)))
    (:then_2
      (for _array_element_3 (Actor|GetComponentsByClass "/Game/Blueprints/Layouts/LayoutLayoutSocket.LayoutLayoutSocket_C")
        (Default|Clear _array_element_3)))))

(fn CheckRecurseAllowed)
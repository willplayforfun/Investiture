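; ObstaclePath is a scene component that spawns a stat-gated obstacle at its transform and tracks the stat levels it sets.
; Jump builds a JumpWall and speed a ClosingDoor, each using a random level clamped to min/max; strength is a stub.
; Recursive getters walk attach-parent ObstaclePaths to sum jump, speed and strength along the chain.
; The last spawned obstacle is stored so ClearObstacle can destroy it.
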(fn BuildJumpObstacle
  (bind _returnvalue (Game|SpawnActorfromClass "/Game/Blueprints/LevelElements/JumpWall.JumpWall_C" (Transformation|GetWorldTransform) "AlwaysSpawn" 0 0))
  (Variables|Default|SetSpawnedObstacle _returnvalue)
  (bind _output_get (Variables|Default|SetCurrentJump (Math|Integer|Min(Integer) (Math|Integer|Max(Integer) (Math|Random|RandomInteger 5) (Variables|Default|GetMinJump self)) (Variables|Default|GetMaxJump self))))
  (Default|BuildforJump _returnvalue _output_get 4.0)
  (return _output_get))

(fn BuildSpeedObstacle
  (bind _returnvalue (Game|SpawnActorfromClass "/Game/Blueprints/LevelElements/ClosingDoor.ClosingDoor_C" (Transformation|GetWorldTransform) "AlwaysSpawn" 0 0))
  (Variables|Default|SetSpawnedObstacle _returnvalue)
  (bind _output_get (Variables|Default|SetCurrentSpeed (Math|Integer|Min(Integer) (Math|Integer|Max(Integer) (Math|Random|RandomInteger 5) (Variables|Default|GetMinSpeed self)) (Variables|Default|GetMaxSpeed self))))
  (Default|SetMinSpeed _returnvalue _output_get)
  (return _output_get))

(fn ClearObstacle
  (bind _spawnedobstacle (Variables|Default|GetSpawnedObstacle))
  (Utilities|IsValid _spawnedobstacle
    (:Is%20Valid
      (Actor|DestroyActor _spawnedobstacle))))

(fn BuildStrengthObstacle
  (return 0))

(fn GetRecursiveStrength
  (bind _path (CallFunction|GetParentPath))
  (Utilities|IsValid _path
    (:Is%20Valid
      (bind _strength (CallFunction|GetRecursiveStrength _path))
      (LocalVariables|SetRecursiveStrength _strength))
    (:Is%20Not%20Valid
      _))
  (return (+ (Variables|Default|GetCurrentStrength) (LocalVariables|GetRecursiveStrength))))

(fn GetRecursiveJump
  (bind _path (CallFunction|GetParentPath))
  (Utilities|IsValid _path
    (:Is%20Valid
      (bind _jump (CallFunction|GetRecursiveJump _path))
      (LocalVariables|SetRecursiveJump _jump))
    (:Is%20Not%20Valid
      _))
  (return (+ (Variables|Default|GetCurrentJump) (LocalVariables|GetRecursiveJump))))

(fn GetRecursiveSpeed
  (bind _path (CallFunction|GetParentPath))
  (Utilities|IsValid _path
    (:Is%20Valid
      (bind _speed (CallFunction|GetRecursiveSpeed _path))
      (LocalVariables|SetRecursiveSpeed _speed))
    (:Is%20Not%20Valid
      _))
  (return (+ (Variables|Default|GetCurrentSpeed) (LocalVariables|GetRecursiveSpeed))))

(fn GetParentPath
  (bind _asobstacle_path (Utilities|Casting|CastToObstaclePath (Transformation|GetAttachParent))
    (:then
      (return _asobstacle_path))
    (:CastFailed
      (return 0))))
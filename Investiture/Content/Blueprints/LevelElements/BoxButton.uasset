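; BoxButton is a level-element button that responds to Cube actors pressing and releasing it.
; It overrides Press and Release to track the IDs of the cubes on it in a Cubes collection.
; When the count reaches one, it turns on its lights and fires activation directly, without calling the parent Press.
; Release passes to the parent only once no cubes remain.
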(event EventBeginPlay
  (|CallParentFunction) ; This node is disabled and will not be called.\nDrag off pins to build functionality.
)

(event EventTick
  (params (DeltaSeconds :type Float%20%28single-precision%29))
  (|CallParentFunction DeltaSeconds) ; This node is disabled and will not be called.\nDrag off pins to build functionality.
)

(event EventPress
  (params (Actor :type Actor%20Object%20Reference))
  (Utilities|Set|Add (Variables|Default|GetCubes) (Variables|/Game/Blueprints/LevelElements/Cube.Cube_C|GetID (.AsCube (Utilities|Casting|CastToCube Actor))))
  (if (== (Utilities|Set|Length (Variables|Default|GetCubes)) 1)
    (CallFunction|SetLights true)
    (Default|CallOnActivate)))

(event EventRelease
  (params (Instantaneous :type Boolean) (LeavingActor :type Actor%20Object%20Reference))
  (Utilities|Set|Remove (Variables|Default|GetCubes) (Variables|/Game/Blueprints/LevelElements/Cube.Cube_C|GetID (.AsCube (Utilities|Casting|CastToCube LeavingActor))))
  (if (== (Utilities|Set|Length (Variables|Default|GetCubes)) 0)
    (|CallParentFunction Instantaneous LeavingActor)))

(fn ConstructionScript
  (|CallParentFunction))
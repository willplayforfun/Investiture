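; Level-element double door that starts open, then closes and reopens as the FirstPersonCharacter overlaps its close and open triggers, gated by a Triggered flag.
; Open and close timelines stop one another and drive SetPos, which slides the two leaves oppositely along an offset relative to their construction-time transforms, scaled by MoveHeight.
; Helper functions reset the door, map a speed index to timeline play rate, and include timer-based cycling and left-leaf collapse logic.
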(event OnComponentBeginOverlap(CloseTrigger)
  (params (OverlappedComponent :type Primitive%20Component%20Object%20Reference) (OtherActor :type Actor%20Object%20Reference) (OtherComp :type Primitive%20Component%20Object%20Reference) (OtherBodyIndex :type Integer) (bFromSweep :type Boolean) (SweepResult :type Hit%20Result%20Structure%20%28by%20ref%29))
  (if (not (Variables|Default|GetTriggered))
    (if (== (Utilities|GetClass OtherActor) "/Game/Blueprints/FirstPersonCharacter.FirstPersonCharacter_C")
      (Variables|Default|SetTriggered true)
      (CallFunction|AnimateClosed))))

(event OnComponentBeginOverlap(OpenTrigger)
  (params (OverlappedComponent :type Primitive%20Component%20Object%20Reference) (OtherActor :type Actor%20Object%20Reference) (OtherComp :type Primitive%20Component%20Object%20Reference) (OtherBodyIndex :type Integer) (bFromSweep :type Boolean) (SweepResult :type Hit%20Result%20Structure%20%28by%20ref%29))
  (if (Variables|Default|GetTriggered)
    (if (== (Utilities|GetClass OtherActor) "/Game/Blueprints/FirstPersonCharacter.FirstPersonCharacter_C")
      (Variables|Default|SetTriggered false)
      (CallFunction|AnimateOpen))))

(event Custom|AnimateOpen
  (Utilities|FlowControl|Sequence
    (:then_0
      (bind _offset (Timeline|CloseTimeline Stop)
        (:Update
          (CallFunction|SetPos _offset))))
    (:then_1
      (bind _offset_2 (Timeline|OpenTimeline PlayFromStart)
        (:Update
          (CallFunction|SetPos _offset_2))))))

(event Custom|AnimateClosed
  (Utilities|FlowControl|Sequence
    (:then_0
      (bind _offset (Timeline|OpenTimeline Stop)
        (:Update
          (CallFunction|SetPos _offset))))
    (:then_1
      (bind _offset_2 (Timeline|CloseTimeline PlayFromStart)
        (:Update
          (CallFunction|SetPos _offset_2))))))

(event EventBeginPlay
  (CallFunction|AnimateOpen))

(event Collision|EventActorBeginOverlap
  (params (OtherActor :type Actor%20Object%20Reference)))

(event EventTick
  (params (DeltaSeconds :type Float%20%28single-precision%29)))

(fn ConstructionScript
  (Variables|Default|SetLeftStartTransform (Transformation|GetWorldTransform (Variables|Default|Getleftdoor)))
  (Variables|Default|SetRightStartTransform (Transformation|GetWorldTransform (Variables|Default|Getrightdoor))))

(fn Collapse
  (if (>= (- (Utilities|Time|GetTimeSeconds) (Variables|Default|GetResetTime)) "0.5f")
    (Class|PrimitiveComponent|SetConstraintMode (Variables|Default|Getleftdoor) "None")
    (Variables|/Script/Engine.PrimitiveComponent|SetCanCharacterStepUpOn (Variables|Default|Getleftdoor) "ECB_No")))

(fn Reset
  (Transformation|SetWorldTransform (Variables|Default|Getleftdoor) (Variables|Default|GetLeftStartTransform) false true)
  (Transformation|SetWorldTransform (Variables|Default|Getrightdoor) (Variables|Default|GetRightStartTransform) false true)
  (Variables|Default|SetTriggered false)
  (Variables|Default|SetResetTime (Utilities|Time|GetTimeSeconds))
  (Audio|Components|Audio|Stop (Variables|Default|GetOpenTimeline))
  (Audio|Components|Audio|Stop (Variables|Default|GetCloseTimeline))
  (CallFunction|AnimateOpen))

(fn MoveDownandUp
  (CallFunction|AnimateOpen)
  (Utilities|Time|SetTimerbyEvent (EventDispatchers|CreateEvent :!event Custom|AnimateClosed) (/ (Variables|Default|GetMovePeriod) 3.0))
  (Utilities|Time|SetTimerbyFunctionName self "MoveDownAndUp" (Variables|Default|GetMovePeriod)))

(fn SetPos
  (params (Offset :type Vector))
  (bind _rightstarttransform (Variables|Default|GetRightStartTransform))
  (bind _leftstarttransform (Variables|Default|GetLeftStartTransform))
  (Utilities|FlowControl|Sequence
    (:then_0
      (Transformation|SetWorldLocation (Variables|Default|Getleftdoor) (+ (Math|Transform|TransformDirection _leftstarttransform (* Offset (Variables|Default|GetMoveHeight))) (.Location (Math|Transform|BreakTransform _leftstarttransform))) false true))
    (:then_1
      (Transformation|SetWorldLocation (Variables|Default|Getrightdoor) (+ (Math|Transform|TransformDirection _rightstarttransform (* Offset (* (Variables|Default|GetMoveHeight) -1.0))) (.Location (Math|Transform|BreakTransform _rightstarttransform))) false true))))

(fn SetMinSpeed
  (params (MinSpeed :type Integer))
  (bind _array (Utilities|Array|MakeArray 0.15 0.3 0.45 0.6 0.75))
  (bind _output (Utilities|Array|Get(acopy) _array MinSpeed))
  (Components|Timeline|SetPlayRate (Variables|Default|GetOpenTimeline) _output)
  (Components|Timeline|SetPlayRate (Variables|Default|GetCloseTimeline) _output))
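; GroundButton is a floor trigger that activates while overlapped by an actor of exactly the AllowType class.
; Overlap begin and end call Press and Release, which toggle four point lights, play sounds and fire activate or deactivate calls.
; CreateArc spawns an Arc aimed at a target point, tinted with the light color while pressed and white otherwise.
; Reset clears Cubes and releases instantly, and destroying the button removes its arc.
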(event OnComponentBeginOverlap(trigger)
  (params (OverlappedComponent :type Primitive%20Component%20Object%20Reference) (OtherActor :type Actor%20Object%20Reference) (OtherComp :type Primitive%20Component%20Object%20Reference) (OtherBodyIndex :type Integer) (bFromSweep :type Boolean) (SweepResult :type Hit%20Result%20Structure%20%28by%20ref%29))
  (if (== (Utilities|GetClass OtherActor) (Variables|Default|GetAllowType))
    (CallFunction|Press OtherActor)
    (Development|PrintString (Utilities|String|Append (Utilities|GetDisplayName OtherComp) " begin overlap"))))

(event OnComponentEndOverlap(trigger)
  (params (OverlappedComponent :type Primitive%20Component%20Object%20Reference) (OtherActor :type Actor%20Object%20Reference) (OtherComp :type Primitive%20Component%20Object%20Reference) (OtherBodyIndex :type Integer))
  (if (== (Utilities|GetClass OtherActor) (Variables|Default|GetAllowType))
    (CallFunction|Release false OtherActor)
    (Development|PrintString (Utilities|String|Append (Utilities|GetDisplayName OtherComp) " end overlap"))))

(event EventBeginPlay
  (CallFunction|SetLights false))

(event EventDestroyed
  (bind _arc (Variables|Default|GetArc))
  (Utilities|IsValid _arc
    (:Is%20Valid
      (Actor|DestroyActor _arc))))

(event EventTick
  (params (DeltaSeconds :type Float%20%28single-precision%29)))

(fn ConstructionScript)

(fn Release
  (params (Instantaneous :type Boolean) (LeavingActor :type Actor%20Object%20Reference))
  (CallFunction|SetLights false)
  (Audio|PlaySoundatLocation (Variables|Default|GetDeactivateSound) (Transformation|GetWorldLocation (Variables|Default|GetArcStart)))
  (Default|CallOnDeactivate Instantaneous))

(fn Reset
  (Utilities|Set|Clear (Variables|Default|GetCubes))
  (CallFunction|Release true))

(fn SetLights
  (params (Visible :type Boolean))
  (Rendering|SetVisibility (Variables|Default|GetPointLight) Visible false)
  (Rendering|SetVisibility (Variables|Default|GetPointLight1) Visible false)
  (Rendering|SetVisibility (Variables|Default|GetPointLight2) Visible false)
  (Rendering|SetVisibility (Variables|Default|GetPointLight3) Visible false)
  (Utilities|IsValid (Variables|Default|GetArc)
    (:Is%20Valid
      (Default|SetColor (Variables|Default|GetArc) (select Visible (Math|Conversions|ToLinearColor(Color) (Variables|/Script/Engine.LightComponentBase|GetLightColor (Variables|Default|GetPointLight))) "(R=1.000000,G=1.000000,B=1.000000,A=1.000000)")))))

(fn Press
  (params (Actor :type Actor%20Object%20Reference))
  (CallFunction|SetLights true)
  (Audio|PlaySoundatLocation (Variables|Default|GetActivateSound) (Transformation|GetWorldLocation (Variables|Default|GetArcStart)))
  (Default|CallOnActivate))

(fn CreateArc
  (params (WorldEnd :type Vector))
  (bind _returnvalue (Transformation|GetActorLocation))
  (bind _returnvalue_2 (- WorldEnd _returnvalue))
  (bind _returnvalue_3 (Game|SpawnActorfromClass "/Game/Blueprints/Arc.Arc_C" (Transformation|GetWorldTransform (Variables|Default|GetArcStart)) "AlwaysSpawn" 0 0))
  (bind _output_get (Variables|Default|SetArc _returnvalue_3))
  (Variables|/Game/Blueprints/Arc.Arc_C|SetDistance _output_get (Math|Vector|VectorLength _returnvalue_2))
  (Transformation|SetActorRotation (Variables|Default|GetArc) (Math|Rotator|FindLookatRotation _returnvalue WorldEnd))
  (Default|BuildArc (Variables|Default|GetArc) (.Z (Math|Vector|BreakVector _returnvalue_2)))
  (Default|SetColor (Variables|Default|GetArc) "(R=1.000000,G=1.000000,B=1.000000,A=1.000000)"))
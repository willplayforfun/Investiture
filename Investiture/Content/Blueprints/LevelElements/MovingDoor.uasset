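; MovingDoor is a level-element door that slides open when enough linked buttons are active and closes when that count drops.
; AttachToButton binds the button's activate and deactivate events, draws an arc to above the door and increments the required count.
; AddButton and SubButton track active buttons against that threshold, triggering Activate or Deactivate.
; These offset the Door instantly by plus or minus MoveDir and play a sound.
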(event EventBeginPlay)

(event Collision|EventActorBeginOverlap
  (params (OtherActor :type Actor%20Object%20Reference)))

(event EventTick
  (params (DeltaSeconds :type Float%20%28single-precision%29)))

(fn ConstructionScript)

(fn AttachtoButton
  (params (Button :type Ground%20Button%20Object%20Reference))
  (Utilities|FlowControl|Sequence
    (:then_0
      (EventDispatchers|BindEventtoOnActivate Button (EventDispatchers|CreateEvent :!event AddButton)))
    (:then_1
      (EventDispatchers|BindEventtoOnDeactivate Button (EventDispatchers|CreateEvent :!event SubButton)))
    (:then_2
      (Default|CreateArc Button (+ (Transformation|GetActorLocation) "0, 0,200.000000"))
      (Math|Integer|IncrementInt (Variables|Default|GetButtonsToOpen)))))

(fn Deactivate
  (params (Instantaneous :type Boolean))
  (Transformation|AddLocalOffset (Variables|Default|Getdoor) (Math|Vector|NegateVector (Variables|Default|GetMoveDir)) false false)
  (Variables|Default|SetActivated false)
  (Audio|PlaySoundatLocation (Variables|Default|GetCloseSound) (Transformation|GetWorldLocation (Variables|Default|Getdoor))))

(fn Activate
  (Transformation|AddLocalOffset (Variables|Default|Getdoor) (Variables|Default|GetMoveDir) false false)
  (Variables|Default|SetActivated true)
  (Audio|PlaySoundatLocation (Variables|Default|GetOpenSound) (Transformation|GetWorldLocation (Variables|Default|Getdoor))))

(fn AddButton
  (bind _result (Math|Integer|IncrementInt (Variables|Default|GetNumActiveButtons))
    (:%20%20
      (bind _output_get (Variables|Default|SetNumActiveButtons _result))
      (if (and (not (Variables|Default|GetActivated)) (>= _output_get (Variables|Default|GetButtonsToOpen)))
        (CallFunction|Activate)))))

(fn SubButton
  (params (Instantaneous :type Boolean))
  (bind _result (Math|Integer|DecrementInt (Variables|Default|GetNumActiveButtons))
    (:%20%20
      (bind _output_get (Variables|Default|SetNumActiveButtons _result))
      (if (and (Variables|Default|GetActivated) (< _output_get (Variables|Default|GetButtonsToOpen)))
        (CallFunction|Deactivate false)))))

(fn ResetRequiredButtons
  (Utilities|FlowControl|Sequence
    (:then_0
      (Variables|Default|SetButtonsToOpen 0))
    (:then_1
      (Variables|Default|SetNumActiveButtons 0))))
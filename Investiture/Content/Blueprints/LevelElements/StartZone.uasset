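; StartZone is a level element actor representing a start area bounded by four static mesh walls.
; SetWallVisibility shows or hides all four meshes together and, when hiding them, plays a leave-zone sound at the actor's root location.
; It has no active event logic of its own, so the function relies on being called from elsewhere.
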(event EventBeginPlay)

(event Collision|EventActorBeginOverlap
  (params (OtherActor :type Actor%20Object%20Reference)))

(event EventTick
  (params (DeltaSeconds :type Float%20%28single-precision%29)))

(fn ConstructionScript)

(fn SetWallVisibility
  (params (Visible :type Boolean))
  (for _array_element (Utilities|Array|MakeArray (Variables|Default|GetStaticMesh2) (Variables|Default|GetStaticMesh3) (Variables|Default|GetStaticMesh4) (Variables|Default|GetStaticMesh1))
    (Rendering|SetVisibility _array_element Visible false))
  (if (not Visible)
    (Audio|PlaySoundatLocation (Variables|Default|GetLeaveZoneSound) (Transformation|GetWorldLocation (Variables|Default|GetDefaultSceneRoot)))))
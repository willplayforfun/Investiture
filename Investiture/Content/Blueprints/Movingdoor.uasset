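; Movingdoor is a door Blueprint that shifts its static mesh when linked to a ground button.
; On BeginPlay it binds events to the activate and deactivate dispatchers of GroundButton, if one is valid.
; Activate offsets the mesh by MoveDir and Deactivate by its negation, each setting the Activated flag.
; Movement is a single unswept jump with no interpolation, and Deactivate ignores its Instantaneous input.
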(event EventBeginPlay
  (bind _groundbutton (Variables|Default|GetGroundButton))
  (Utilities|IsValid _groundbutton
    (:Is%20Valid
      (CallFunction|AttachtoButton _groundbutton))))

(event Collision|EventActorBeginOverlap
  (params (OtherActor :type Actor%20Object%20Reference)))

(event EventTick
  (params (DeltaSeconds :type Float%20%28single-precision%29)))

(fn ConstructionScript)

(fn AttachtoButton
  (params (Button :type Ground%20Button%20Object%20Reference))
  (Utilities|FlowControl|Sequence
    (:then_0
      (EventDispatchers|BindEventtoOnActivate Button (EventDispatchers|CreateEvent :!event Activate)))
    (:then_1
      (EventDispatchers|BindEventtoOnDeactivate Button (EventDispatchers|CreateEvent :!event Deactivate)))))

(fn Deactivate
  (params (Instantaneous :type Boolean))
  (Transformation|AddLocalOffset (Variables|Default|GetStaticMesh) (Math|Vector|NegateVector (Variables|Default|GetMoveDir)) false false)
  (Variables|Default|SetActivated false))

(fn Activate
  (Transformation|AddLocalOffset (Variables|Default|GetStaticMesh) (Variables|Default|GetMoveDir) false false)
  (Variables|Default|SetActivated true))
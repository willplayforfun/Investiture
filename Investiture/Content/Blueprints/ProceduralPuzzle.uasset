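; ProceduralPuzzle manages puzzle level setup and reset.
; On BeginPlay it caches all CubeSpawners, the first StartZone and all CollapsingPlatforms, then runs ResetLevel to reset spawners and platforms and show the start zone walls.
; GenerateLevel, not called within this graph, prints the level number and fills PuzzleGameState's total and free Speed, Jump and Strength with fixed values, regardless of that number.
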(event EventBeginPlay
  (Utilities|FlowControl|Sequence
    (:then_0
      (bind _outactors (Actor|GetAllActorsOfClass "/Game/Blueprints/CubeSpawner.CubeSpawner_C"))
      (Variables|Default|SetCubeSpawners _outactors))
    (:then_1
      (bind _outactors_2 (Actor|GetAllActorsOfClass "/Game/LevelElements/StartZone.StartZone_C"))
      (Variables|Default|SetStartZone (Utilities|Array|Get(acopy) _outactors_2)))
    (:then_2
      (bind _outactors_3 (Actor|GetAllActorsOfClass "/Game/Blueprints/CollapsingPlatform.CollapsingPlatform_C"))
      (Variables|Default|SetCollapsingPlatforms _outactors_3))
    (:then_3
      (CallFunction|ResetLevel))))

(event Collision|EventActorBeginOverlap
  (params (OtherActor :type Actor%20Object%20Reference)))

(event EventTick
  (params (DeltaSeconds :type Float%20%28single-precision%29)))

(fn ConstructionScript)

(fn GenerateLevel
  (params (Num :type Integer))
  (Development|PrintString (Utilities|String|Append "Creating Level " (Utilities|String|ToString(Integer) Num)))
  (bind _aspuzzle_game_state (Utilities|Casting|CastToPuzzleGameState (Game|GetGameState)))
  (Utilities|FlowControl|Sequence
    (:then_0
      (bind _output_get (Variables|/Game/Blueprints/PuzzleGameState.PuzzleGameState_C|SetTotalSpeed _aspuzzle_game_state 4))
      (Variables|/Game/Blueprints/PuzzleGameState.PuzzleGameState_C|SetFreeSpeed _aspuzzle_game_state _output_get))
    (:then_1
      (bind _output_get_2 (Variables|/Game/Blueprints/PuzzleGameState.PuzzleGameState_C|SetTotalJump _aspuzzle_game_state 4))
      (Variables|/Game/Blueprints/PuzzleGameState.PuzzleGameState_C|SetFreeJump _aspuzzle_game_state _output_get_2))
    (:then_2
      (bind _output_get_3 (Variables|/Game/Blueprints/PuzzleGameState.PuzzleGameState_C|SetTotalStrength _aspuzzle_game_state 0))
      (Variables|/Game/Blueprints/PuzzleGameState.PuzzleGameState_C|SetFreeStrength _aspuzzle_game_state _output_get_3))))

(fn ResetLevel
  (Utilities|FlowControl|Sequence
    (:then_0
      (for _array_element (Variables|Default|GetCubeSpawners)
        (Default|Reset _array_element)))
    (:then_1
      (Default|SetWallVisibility (Variables|Default|GetStartZone) true))
    (:then_2
      (for _array_element_2 (Variables|Default|GetCollapsingPlatforms)
        (Default|Reset _array_element_2)))))
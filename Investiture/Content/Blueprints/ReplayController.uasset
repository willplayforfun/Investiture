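; Controller that replays a recorded run on a possessed FirstPersonCharacter, shown in third person and tinted by its visible index.
; Tick advances at most one recorded frame as replay time passes the summed deltas, teleporting the pawn and adding spline points.
; Timestamped grabs and throws replay alternately through a shared index, with cubes matched by ID.
; Overview mode adds a stats widget, and Delete has the owning controller destroy the run.
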(event EventBeginPlay)

(event EventTick
  (params (DeltaSeconds :type Float%20%28single-precision%29))
  (bind _rotations (Variables|Default|GetRotations))
  (bind _grabthrowindex (Variables|Default|GetGrabThrowIndex))
  (bind _positions (Variables|Default|GetPositions))
  (bind _throws (Variables|Default|GetThrows))
  (bind _grabthrowindex_2 (Variables|Default|GetGrabThrowIndex))
  (bind _grabs (Variables|Default|GetGrabs))
  (bind _output (Utilities|Array|Get(acopy) _throws _grabthrowindex_2))
  (bind _output_2 (Utilities|Array|Get(acopy) _grabs _grabthrowindex))
  (bind (_time _id _position) (Utilities|Struct|BreakPickupEvent _output_2))
  (bind (_time_2 _position_2 _rotation) (Utilities|Struct|BreakThrowEvent _output))
  (if (Variables|Default|GetReplaying)
    (bind _output_get (Variables|Default|SetReplayTime (+ (Variables|Default|GetReplayTime) DeltaSeconds)))
    (if (< (Variables|Default|GetCumDeltas) _output_get)
      (bind _result (Math|Integer|IncrementInt (Variables|Default|GetCurrentIndex))
        (:%20%20
          (if (> (Utilities|Array|Length (Variables|Default|GetDeltas)) _result)
            ;[1 1 1] PlayNextFrame
            (Variables|Default|SetCumDeltas (+ (Utilities|Array|Get(acopy) (Variables|Default|GetDeltas) (Variables|Default|GetCurrentIndex)) (Variables|Default|GetCumDeltas)))
            (Transformation|SetActorLocation (Pawn|GetControlledPawn) (Utilities|Array|Get(acopy) (Variables|Default|GetPositions) (Variables|Default|GetCurrentIndex)) false true)
            (Transformation|SetActorRotation (Pawn|GetControlledPawn) (Utilities|Array|Get(acopy) (Variables|Default|GetRotations) (Variables|Default|GetCurrentIndex)) true)
            (bind _asfirst_person_character (Utilities|Casting|CastToFirstPersonCharacter (Pawn|GetControlledPawn)))
            (Default|AddSplinePoint _asfirst_person_character 0.0)
            (if (Variables|Default|GetGrabbing)
              (if (> (Utilities|Array|Length (Variables|Default|GetThrows)) (Variables|Default|GetGrabThrowIndex))
                (if (<= _time_2 (Variables|Default|GetReplayTime))
                  (Default|Throw (.AsFirst%20Person%20Character (Utilities|Casting|CastToFirstPersonCharacter (Pawn|GetControlledPawn))) _position_2 _rotation true 0.0)
                  (Math|Integer|IncrementInt (Variables|Default|GetGrabThrowIndex)
                    (:%20%20
                      (Variables|Default|SetGrabbing false)))))
              (elif (> (Utilities|Array|Length (Variables|Default|GetGrabs)) (Variables|Default|GetGrabThrowIndex))
                (if (<= _time (Variables|Default|GetReplayTime))
                  (Variables|Default|SetGrabbing true)
                  (bind _outactors (Actor|GetAllActorsOfClass "/Game/Blueprints/Cube.Cube_C"))
                  (bind _array_element (Utilities|Array|ForEachLoopwithBreak _outactors :!label _label)
                    (:LoopBody
                      (if (and (not (Variables|/Game/Blueprints/Cube.Cube_C|GetisGrabbed _array_element)) (== (Variables|/Game/Blueprints/Cube.Cube_C|GetID _array_element) _id))
                        (Default|Grab (.AsFirst%20Person%20Character (Utilities|Casting|CastToFirstPersonCharacter (Pawn|GetControlledPawn))) _array_element _position true)
                        (goto _label Break)))))))
            (else
              (Transformation|SetActorLocation (Pawn|GetControlledPawn) (Utilities|Array|Get(acopy) _positions (Utilities|Array|LastIndex _positions)) false true)
              (Transformation|SetActorRotation (Pawn|GetControlledPawn) (Utilities|Array|Get(acopy) _rotations (Utilities|Array|LastIndex _rotations)) true))))))))

(fn ConstructionScript)

(fn StartReplay
  (params (Run :type Player%20Run%20Structure) (ControllerRef :type First%20Person%20Controller%20Object%20Reference) (RunIndex :type Integer) (Overview :type Boolean) (VisibleIndex :type Integer))
  (bind (_positions _rotations _deltas _speed _jump _strength _deleted _recordedthrows _recordedgrabs) (Utilities|Struct|BreakPlayerRun Run))
  (bind _returnvalue (Math|Color|MakeColor 0.0 255.0 0.0 255.0))
  (bind _returnvalue_2 (Math|Color|MakeColor 0.0 0.0 255.0 255.0))
  (bind _returnvalue_3 (Math|Color|MakeColor 255.0 0.0 255.0 255.0))
  (bind _returnvalue_4 (Math|Color|MakeColor 255.0 255.0 0.0 255.0))
  (bind _returnvalue_5 (Math|Color|MakeColor 0.0 255.0 255.0 255.0))
  (bind _returnvalue_6 (Math|Color|MakeColor 255.0 0.0 0.0 255.0))
  (bind _array (Utilities|Array|MakeArray _returnvalue_6 _returnvalue _returnvalue_2 _returnvalue_3 _returnvalue_4 _returnvalue_5))
  (bind _output (Utilities|Array|Get(acopy) _array VisibleIndex))
  (Default|Set3P (.AsFirst%20Person%20Character (Utilities|Casting|CastToFirstPersonCharacter (Pawn|GetControlledPawn))) true)
  (LocalVariables|SetOverviewView Overview)
  (Variables|Default|SetControllerRef ControllerRef)
  (Variables|Default|SetRunIndex RunIndex)
  (Variables|Default|SetReplayTime 0.0)
  (Variables|Default|SetReplayStartTime (Utilities|Time|GetGameTimeinSeconds))
  (Variables|Default|SetPositions _positions)
  (Variables|Default|SetRotations _rotations)
  (Variables|Default|SetDeltas _deltas)
  (LocalVariables|SetSpeed _speed)
  (LocalVariables|SetJump _jump)
  (LocalVariables|SetStrength _strength)
  (Variables|Default|SetThrows _recordedthrows)
  (Variables|Default|SetGrabs _recordedgrabs)
  (Variables|Default|SetGrabThrowIndex 0)
  (Variables|Default|SetReplaying true)
  (Variables|Default|SetCurrentIndex -1)
  (Variables|Default|SetCumDeltas 0.0)
  (Variables|Default|SetColorIndex VisibleIndex)
  (Default|SetColor (.AsFirst%20Person%20Character (Utilities|Casting|CastToFirstPersonCharacter (Pawn|GetControlledPawn))) _output)
  (if (LocalVariables|GetOverviewView)
    (bind _returnvalue_7 (UserInterface|CreateWidget "/Game/Blueprints/ReplayStatsWidget.ReplayStatsWidget_C" (Game|GetPlayerController 0)))
    (bind _output_get (Variables|Default|SetStatsBar _returnvalue_7))
    (UserInterface|Viewport|AddtoViewport _returnvalue_7 0)
    (Default|SetPawnTarget _returnvalue_7 (Pawn|GetControlledPawn))
    (Default|SetValues _returnvalue_7 (LocalVariables|GetSpeed) (LocalVariables|GetJump) (LocalVariables|GetStrength))
    (return (Variables|Default|GetRunIndex) _output)))

(fn Delete
  (bind _statsbar (Variables|Default|GetStatsBar))
  (Default|DestroyRun (Variables|Default|GetControllerRef) (Variables|Default|GetRunIndex))
  (Utilities|IsValid _statsbar
    (:Is%20Valid
      (Widget|RemovefromParent _statsbar))))

(fn StopReplay
  (bind _statsbar (Variables|Default|GetStatsBar))
  (Utilities|IsValid _statsbar
    (:Is%20Valid
      (Widget|RemovefromParent _statsbar))))
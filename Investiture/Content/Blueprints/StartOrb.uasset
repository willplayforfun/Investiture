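; StartOrb is an orb actor with a sphere mesh, a particle effect and a text render component.
; SetColor creates a dynamic material instance on the sphere and applies the given color to both its Color parameter and the particles' Color parameter.
; The event graph and construction script do nothing; unconnected nodes meant to rotate the text from a look-at toward the player pawn never run.
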(event EventBeginPlay)

(event Collision|EventActorBeginOverlap
  (params (OtherActor :type Actor%20Object%20Reference)))

(event EventTick
  (params (DeltaSeconds :type Float%20%28single-precision%29)))

(fn ConstructionScript)

(fn SetColor
  (params (Color :type Linear%20Color%20Structure))
  (bind _sphere (Variables|Default|GetSphere))
  (bind _returnvalue (Rendering|Material|CreateDynamicMaterialInstance _sphere 0 (Rendering|Material|GetMaterial _sphere 0) :!class /Script/Engine.PrimitiveComponent))
  (Rendering|Material|SetVectorParameterValue _returnvalue "Color" Color :!class /Script/Engine.MaterialInstanceDynamic)
  (Effects|Components|ParticleSystem|SetColorParameter (Variables|Default|GetStartOrbParticles) "Color" Color))